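; BP_GameMode is the game mode Blueprint that brings up the game's UI at level start.
; On BeginPlay it gets the first player controller, shows the mouse cursor and pauses the game.
; It then creates the BP_Menu and BP_Pause widgets, hands each the controller and adds both to the viewport.
; Tick and the construction script are empty, and nothing here unpauses the game.
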(event EventBeginPlay
  (bind _output_get (Variables|Default|SetPlayer (Game|GetPlayerController 0)))
  (Variables|/Script/Engine.PlayerController|SetbShowMouseCursor _output_get true)
  (Game|SetGamePaused true)
  (bind _returnvalue (UserInterface|CreateWidget "/Game/BP/BP_Menu.BP_Menu_C"))
  (Variables|/Game/BP/BP_Menu.BP_Menu_C|SetPlayer _returnvalue (Variables|Default|GetPlayer))
  (UserInterface|Viewport|AddtoViewport _returnvalue 0)
  (bind _returnvalue_2 (UserInterface|CreateWidget "/Game/BP/BP_Pause.BP_Pause_C"))
  (Variables|/Game/BP/BP_Pause.BP_Pause_C|SetPlayer _returnvalue_2 (Variables|Default|GetPlayer))
  (UserInterface|Viewport|AddtoViewport _returnvalue_2 0))

(event EventTick
  (params (DeltaSeconds :type Float%20%28single-precision%29)))

(fn ConstructionScript)