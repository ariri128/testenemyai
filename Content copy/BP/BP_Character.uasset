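; BP_Character is a player character Blueprint that provides basic movement and look controls through Enhanced Input.
; On BeginPlay it adds the IMC_baseCharacter mapping context to player controller 0's input subsystem.
; Locomotion and strafe actions add movement input along the actor's forward and right vectors.
; Vertical and horizontal look actions feed controller pitch and yaw directly, with no additional scaling.
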(event Input|EnhancedActionEvents|EnhancedInputActionIA_Locamotion
  (params (ActionValue :type Float%20%28double-precision%29) (ElapsedSeconds :type Float%20%28double-precision%29) (TriggeredSeconds :type Float%20%28double-precision%29) (InputAction :type Input%20Action%20Object%20Reference :default "/Game/BP/UI/IO/IA_Locamotion.IA_Locamotion"))
  ;[0.15 0.15 0.15 0.5] Basic Features
  (Pawn|Input|AddMovementInput (Transformation|GetActorForwardVector) ActionValue false))

(event Input|EnhancedActionEvents|EnhancedInputActionIA_LookH
  (params (ActionValue :type Float%20%28double-precision%29) (ElapsedSeconds :type Float%20%28double-precision%29) (TriggeredSeconds :type Float%20%28double-precision%29) (InputAction :type Input%20Action%20Object%20Reference :default "/Game/BP/UI/IO/IA_LookH.IA_LookH"))
  ;[0.15 0.15 0.15 0.5] Basic Features
  (Pawn|Input|AddControllerYawInput ActionValue))

(event Input|EnhancedActionEvents|EnhancedInputActionIA_LookV
  (params (ActionValue :type Float%20%28double-precision%29) (ElapsedSeconds :type Float%20%28double-precision%29) (TriggeredSeconds :type Float%20%28double-precision%29) (InputAction :type Input%20Action%20Object%20Reference :default "/Game/BP/UI/IO/IA_LookV.IA_LookV"))
  ;[0.15 0.15 0.15 0.5] Basic Features
  (Pawn|Input|AddControllerPitchInput ActionValue))

(event Input|EnhancedActionEvents|EnhancedInputActionIA_Strafe
  (params (ActionValue :type Float%20%28double-precision%29) (ElapsedSeconds :type Float%20%28double-precision%29) (TriggeredSeconds :type Float%20%28double-precision%29) (InputAction :type Input%20Action%20Object%20Reference :default "/Game/BP/UI/IO/IA_Strafe.IA_Strafe"))
  ;[0.15 0.15 0.15 0.5] Basic Features
  (Pawn|Input|AddMovementInput (Transformation|GetActorRightVector) ActionValue false))

(event EventBeginPlay
  ;[0.15 0.15 0.15 0.5] Establish IMC Mapping
  (Input|AddMappingContext (PlayerController|LocalPlayerSubsystems|GetEnhancedInputLocalPlayerSubsystem (Game|GetPlayerController 0)) "/Game/BP/UI/IO/IMC_baseCharacter.IMC_baseCharacter" 0 "(bIgnoreAllPressedKeysUntilRelease=True,bForceImmediately=False,bNotifyUserSettings=False)"))

(fn ConstructionScript)